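; Player Blueprint for a wave-based shooter, handling movement, turning toward a supplied target, hitscan shooting and limited rockets.
; Enhanced Input drives movement and both attacks: a line trace applies point damage, while rockets spawn as actors.
; Damage drains shield before health, and Tick refills shield by a per-frame step after a damage-free delay.
; It pushes stat changes to WB_HUD and counts waves via the GameMode's wave-end binding.
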(event Custom|WaveEnd
  (Default|HealthUpdateUI (Variables|Default|GetHUD) (Variables|Default|GetcurrentHealth) (Variables|Default|GetmaxHealth))
  (Default|RocketUpgradeUI (Variables|Default|GetHUD) (Variables|Default|GetRocket) (Variables|Default|GetmaxRocket))
  (bind _result (Math|Float|IncrementFloat (Variables|Default|GetWave))
    (:%20%20
      (bind _output_get (Variables|Default|SetWave _result))
      (Development|PrintString (Utilities|String|ToString(Float) _output_get))
      (Default|WaveUpdateUI (Variables|Default|GetHUD) _output_get))))

(event Input|EnhancedActionEvents|EnhancedInputActionIA_Shoot
  (params (ActionValue :type Boolean) (ElapsedSeconds :type Float%20%28double-precision%29) (TriggeredSeconds :type Float%20%28double-precision%29) (InputAction :type Input%20Action%20Object%20Reference :default "/Game/Player/Input/Actions/IA_Shoot.IA_Shoot"))
  (bind _shoot_point (Variables|Default|GetShoot%20Point))
  (bind _returnvalue (Transformation|GetWorldLocation _shoot_point))
  ;[0 0 0] Attack
  (:Started
    (bind _outhit (Collision|LineTraceByChannel _returnvalue (+ _returnvalue (* (Math|Vector|GetForwardVector _shoot_point) (Variables|Default|GetBullet%20Range))) "TraceTypeQuery1" false 0 "ForDuration"))
    (Game|Damage|ApplyPointDamage (.hitactor _outhit) 1e+01 (.location _outhit) (Collision|MakeHitResult false false 0.0 0.0 "0, 0, 0" "0, 0, 0" "0,0,1" "0,0,1" 0 0))))

(event Input|EnhancedActionEvents|EnhancedInputActionIA_Movement
  (params (ActionValue :type Vector%202D%20Structure) (ElapsedSeconds :type Float%20%28double-precision%29) (TriggeredSeconds :type Float%20%28double-precision%29) (InputAction :type Input%20Action%20Object%20Reference :default "/Game/Player/Input/Actions/IA_Movement.IA_Movement"))
  (bind _returnvalue (Pawn|GetControlRotation :!class /Script/Engine.Pawn))
  (bind _returnvalue_2 (Math|Rotator|MakeRotator (.yaw _returnvalue) 0.0 (.yaw _returnvalue)))
  ;[0 0 0] Movement
  (Utilities|FlowControl|Sequence
    (:then_0
      (Pawn|Input|AddMovementInput (Math|Vector|GetForwardVector _returnvalue_2) (.x ActionValue) false))
    (:then_1
      (Pawn|Input|AddMovementInput (Math|Vector|GetRightVector _returnvalue_2) (.y ActionValue) false))))

(event Input|EnhancedActionEvents|EnhancedInputActionIA_Special
  (params (ActionValue :type Boolean) (ElapsedSeconds :type Float%20%28double-precision%29) (TriggeredSeconds :type Float%20%28double-precision%29) (InputAction :type Input%20Action%20Object%20Reference :default "/Game/Player/Input/Actions/IA_Special.IA_Special"))
  ;[0 0 0] Rocket
  (:Started
    (if (> (Variables|Default|GetRocket) 0.0)
      (Variables|Default|SetRocket (- (Variables|Default|GetRocket) 1.0))
      (Game|SpawnActorfromClass "/Game/Player/Blueprints/Special/BP_Rocket.BP_Rocket_C" (Transformation|GetWorldTransform (Variables|Default|GetArrow1)) "Undefined" "MultiplyWithRoot" 0 0)
      (Variables|Default|SetLastRocket (Utilities|Time|GetGameTimeinSeconds))
      (Default|RocketUpgradeUI (Variables|Default|GetHUD) (Variables|Default|GetRocket) (Variables|Default|GetmaxRocket)))))

(event EventBeginPlay
  (Input|AddMappingContext (PlayerController|LocalPlayerSubsystems|GetEnhancedInputLocalPlayerSubsystem (Game|GetPlayerController 0)) "/Game/Player/Input/IMC_Player.IMC_Player" 0 "(bIgnoreAllPressedKeysUntilRelease=True,bForceImmediately=False,bNotifyUserSettings=False)")
  (bind _returnvalue (UserInterface|CreateWidget "/Game/UI/WB_HUD.WB_HUD_C" (Game|GetPlayerController 0)))
  (bind _output_get (Variables|Default|SetHUD _returnvalue))
  (UserInterface|Viewport|AddtoViewport _output_get 0)
  (Variables|Default|SetcurrentHealth (Variables|Default|GetmaxHealth))
  (Variables|Default|SetcurrentShield (Variables|Default|GetmaxShield))
  (Variables|Default|SetRocket (Variables|Default|GetmaxRocket))
  (bind _asbp_third_person_game_mode (Utilities|Casting|CastToBP_ThirdPersonGameMode (Game|GetGameMode)))
  (bind _output_get_2 (Variables|Default|SetAs%20BP%20Third%20Person%20Game%20Mode _asbp_third_person_game_mode))
  (EventDispatchers|BindEventtoWaveEnd _output_get_2 (delegate Custom|WaveEnd)))

(event Game|Damage|EventAnyDamage
  (params (Damage :type Float%20%28single-precision%29) (DamageType :type Damage%20Type%20Object%20Reference) (InstigatedBy :type Controller%20Object%20Reference) (DamageCauser :type Actor%20Object%20Reference))
  ;[0 0 0] Health/Shield
  ;;[0 0.552 1] Shield Status
  (Utilities|FlowControl|Sequence
    (:then_0
      (if (<= (Variables|Default|GetcurrentShield) 0.0)
        (Variables|Default|SetnoShield true)
        (else
          (Variables|Default|SetnoShield false))))
    (:then_1
      ;;[0 0.361 1] Shield Damage
      (Variables|Default|SetlastDamageTime (Utilities|Time|GetGameTimeinSeconds))
      (if (not (Variables|Default|GetnoShield))
        (bind _output_get (Variables|Default|SetcurrentShield (Math|Float|Clamp(Float) (- (Variables|Default|GetcurrentShield) Damage) 0.0 (Variables|Default|GetmaxShield))))
        (Default|ShieldUpdateUI (Variables|Default|GetHUD) _output_get (Variables|Default|GetmaxShield))
        (else
          ;;[1 0 0] Health Damage
          (bind _output_get_2 (Variables|Default|SetcurrentHealth (Math|Float|Clamp(Float) (- (Variables|Default|GetcurrentHealth) Damage) 0.0 (Variables|Default|GetmaxHealth))))
          (Default|HealthUpdateUI (Variables|Default|GetHUD) _output_get_2 (Variables|Default|GetmaxHealth)))))))

(event EventLookat
  (params (Target :type Vector :default "0, 0, 0"))
  (bind _returnvalue (Transformation|GetActorLocation))
  ;[0 0 0] Look At Mouse
  (Transformation|SetActorRotation (Math|Rotator|FindLookatRotation (Math|Vector|MakeVector (.x _returnvalue) (.y _returnvalue) 0.0) (Math|Vector|MakeVector (.x Target) (.y Target) 0.0))))

(event EventTick
  (params (DeltaSeconds :type Float%20%28single-precision%29))
  ;[0 0 0] Health/Shield
  ;;[0 0.283 1] Shield Recharge
  (if (>= (- (Utilities|Time|GetGameTimeinSeconds) (Variables|Default|GetlastDamageTime)) (Variables|Default|GetregenDelay))
    (if (< (Variables|Default|GetcurrentShield) (Variables|Default|GetmaxShield))
      (bind _output_get (Variables|Default|SetcurrentShield (+ (Variables|Default|GetcurrentShield) (Variables|Default|GetshieldRegenRate))))
      (Default|ShieldUpdateUI (Variables|Default|GetHUD) _output_get (Variables|Default|GetmaxShield)))))

(fn ConstructionScript)