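; Enemy actor that chases the player, plays a melee attack montage and dies when its health runs out.
; Every Tick it issues AIMoveTo toward the cached player controller, not the pawn; on arrival a CanAttack flag gates the montage for its duration.
; A Box overlap with BP_Player applies damage independently of the attack state.
; Incoming damage lowers clamped Health, firing OnEnemyKilled before destruction at zero.
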(event OnComponentBeginOverlap(Box)
  (params (OverlappedComponent :type Primitive%20Component%20Object%20Reference) (OtherActor :type Actor%20Object%20Reference) (OtherComp :type Primitive%20Component%20Object%20Reference) (OtherBodyIndex :type Integer) (bFromSweep :type Boolean) (SweepResult :type Hit%20Result%20Structure%20%28by%20ref%29))
  (Utilities|Casting|CastToBP_Player OtherActor)
  (Development|PrintString "overlap")
  (Game|Damage|ApplyDamage OtherActor 1e+01 0 0))

(event Custom|Follow%20Player
  (AI|AIMoveTo self "0, 0, 0" (Variables|Default|GetAs%20BP%20Player%20Controller) 7e+01 false
    (:OnSuccess
      (if (Variables|Default|GetcanAttack)
        (Variables|Default|SetcanAttack false)
        (bind _returnvalue (Animation|PlayAnimMontage "/Game/Characters/Enemy/AM_Enemy.AM_Enemy" 1.0 "None"))
        (Utilities|FlowControl|Delay _returnvalue)
        (Variables|Default|SetcanAttack true)))))

(event EventBeginPlay
  (bind _asbp_player_controller (Utilities|Casting|CastToBP_PlayerController (Game|GetPlayerController 0)))
  (Variables|Default|SetAs%20BP%20Player%20Controller _asbp_player_controller)
  (Variables|Default|SetHealth (Variables|Default|GetMaxHealth)))

(event Game|Damage|EventAnyDamage
  (params (Damage :type Float%20%28single-precision%29) (DamageType :type Damage%20Type%20Object%20Reference) (InstigatedBy :type Controller%20Object%20Reference) (DamageCauser :type Actor%20Object%20Reference))
  (Variables|Default|SetHealth (Math|Float|Clamp(Float) (- (Variables|Default|GetHealth) Damage) 0.0 3e+01))
  (if (<= (Variables|Default|GetHealth) 0.0)
    (Default|CallOnEnemyKilled)
    (Actor|DestroyActor)))

(event EventTick
  (params (DeltaSeconds :type Float%20%28single-precision%29))
  (CallFunction|FollowPlayer))

(fn ConstructionScript)