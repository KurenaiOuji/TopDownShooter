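; BP_Spawn is an enemy spawn point that creates BP_Enemy actors at its own transform.
; On BeginPlay, each instance picks a random BP_Spawn in the level and calls its SpawnEnemy directly, bypassing the enemy cap.
; The Spawn event calls SpawnEnemy only while the current count is below the maximum.
; SpawnEnemy requires BP_ThirdPersonGameMode, then spawns the enemy, increments the count and prints it.
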(event Custom|Spawn
  (if (< (Variables|Default|GetCurrentEnemyCount) (Variables|Default|GetMaxEnemies))
    (CallFunction|SpawnEnemy)))

(event EventBeginPlay
  (bind _outactors (Actor|GetAllActorsOfClass "BP_Spawn_C"))
  (CallFunction|SpawnEnemy (.OutItem (Utilities|Array|Random _outactors))))

(fn ConstructionScript)

(fn SpawnEnemy
  (bind _asbp_third_person_game_mode (Utilities|Casting|CastToBP_ThirdPersonGameMode (Game|GetGameMode)))
  (Variables|Default|SetAs%20BP%20Third%20Person%20Game%20Mode _asbp_third_person_game_mode)
  (if true
    (Game|SpawnActorfromClass "/Game/Enemy/Blueprints/BP_Enemy.BP_Enemy_C" (Transformation|GetActorTransform) "Undefined" "MultiplyWithRoot" 0 0)
    (bind _output_get (Variables|Default|SetCurrentEnemyCount (+ (Variables|Default|GetCurrentEnemyCount) (Variables|Default|GetIncrementEnemyCount%20))))
    (Development|PrintString (Utilities|String|ToString(Integer) _output_get))))